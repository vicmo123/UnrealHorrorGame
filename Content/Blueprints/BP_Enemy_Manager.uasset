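; BP_Enemy_Manager is a central manager that caps how many BP_Enemy_AI enemies exist at once.
; On BeginPlay it registers itself with every BP_Enemy_Spawn_Point in the level.
; RequestSpawn checks the live count against the maximum, spawns at the given transform and adds the enemy to a tracking array, while RemoveEnemyArray frees a slot.
; Tick prints the tracked enemy count on screen for debugging.
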(event Custom|RequestSpawn
  (params (SpawnLocation :type Transform))
  (bind _canspawn (CallFunction|CheckifCanSpawn))
  (if _canspawn
    (bind _newenemy (CallFunction|SpawnNewEnemy SpawnLocation))
    (CallFunction|AddEnemyArray _newenemy)))

(event EventTick
  (params (DeltaSeconds :type Float%20%28single-precision%29))
  (Development|PrintText (Utilities|Text|ToText(Integer) (Utilities|Array|Length (Variables|Default|GetEnemyArray))) true false "(R=0.000000,G=0.781802,B=1.000000,A=1.000000)" -1.0 "SpawnedEnemies"))

(event EventBeginPlay
  (bind _outactors (Actor|GetAllActorsOfClass "/Game/Blueprints/BP_Enemy_Spawn_Point.BP_Enemy_Spawn_Point_C"))
  (for _array_element _outactors
    (Variables|/Game/Blueprints/BP_Enemy_Spawn_Point.BP_Enemy_Spawn_Point_C|SetEnemyManager _array_element self)))

(fn ConstructionScript)

(fn SpawnNewEnemy
  (params (SpawnTransform :type Transform))
  (bind _returnvalue (Game|SpawnActorfromClass "/Game/Blueprints/BP_Enemy_AI.BP_Enemy_AI_C" SpawnTransform "Undefined" "MultiplyWithRoot" 0 0))
  (return _returnvalue))

(fn CheckifCanSpawn
  (if (< (Variables|Default|GetNumberSpawnedEnemies) (Variables|Default|GetMaxNumberEnemies))
    (return true)
    (else
      (Development|PrintText "No More Enemies Can Spawn Right Now")
      (return false))))

(fn AddEnemyArray
  (params (NewEnemy :type BP%20Enemy%20AI%20Object%20Reference))
  (Utilities|Array|Add (Variables|Default|GetEnemyArray) NewEnemy)
  (Math|Integer|IncrementInt (Variables|Default|GetNumberSpawnedEnemies)))

(fn RemoveEnemyArray
  (params (EnemyToRemove :type BP%20Enemy%20AI%20Object%20Reference))
  (Utilities|Array|RemoveItem (Variables|Default|GetEnemyArray) EnemyToRemove)
  (Math|Integer|DecrementInt (Variables|Default|GetNumberSpawnedEnemies)))