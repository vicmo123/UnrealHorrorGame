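; Enemy spawn point that requests a wave of enemies from the EnemyManager when the main character enters its trigger box.
; Each overlap while armed sends one spawn request per wave enemy, all at the Spawn component's transform, leaving the manager to enforce the enemy limit.
; A Tick-driven timer re-arms the zone after TimeBeforeReset.
; The construction script applies the configurable trigger size and spawn offset.
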(event OnComponentBeginOverlap(TriggerZone)
  (params (OverlappedComponent :type Primitive%20Component%20Object%20Reference) (OtherActor :type Actor%20Object%20Reference) (OtherComp :type Primitive%20Component%20Object%20Reference) (OtherBodyIndex :type Integer) (bFromSweep :type Boolean) (SweepResult :type Hit%20Result%20Structure%20%28by%20ref%29))
  ;[1 1 1] If detection is detected and the time is right, it will request spawn to the enemy manager wich will check if it can be spawned according to the max number of enemies, it will the create one and add it to an array.
  (Utilities|Casting|CastToBP_Main_Character OtherActor)
  (if (not (Variables|Spawning|GetEnemiesHaveBeenSpawned))
    (Variables|Spawning|SetEnemiesHaveBeenSpawned true)
    (for _index (range 0 (- (Variables|Spawning|GetNumEnemiesPerWave) 1))
      (Default|RequestSpawn (Variables|Spawning|GetEnemyManager) (Transformation|GetWorldTransform (Variables|Default|GetSpawn))))))

(event Custom|UpdateTimer
  (params (DeltaTime :type Float%20%28double-precision%29))
  ;[1 1 1] Reset Timer - timer that counts up from the time the zone is triggered, when it is up, it invoked the reset, wich allows to retrigger the spawn zone.
  (if (Variables|Spawning|GetEnemiesHaveBeenSpawned)
    (Variables|Spawning|SetCurrentTime (+ DeltaTime (Variables|Spawning|GetCurrentTime)))
    (if (>= (Variables|Spawning|GetCurrentTime) (Variables|Spawning|GetTimeBeforeReset))
      (Variables|Spawning|SetEnemiesHaveBeenSpawned false)
      (Variables|Spawning|SetCurrentTime 0.0))))

(event EventTick
  (params (DeltaSeconds :type Float%20%28single-precision%29))
  (CallFunction|UpdateTimer DeltaSeconds))

(fn ConstructionScript
  (Transformation|AddLocalOffset (Variables|Default|GetSpawn) (Variables|Spawning|GetSpawnLocation) false false)
  (Components|Box|SetBoxExtent (Variables|Default|GetTriggerZone) (Variables|Spawning|GetTriggerZoneSize) true))