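; Enemy AI character that chases the player on sight and fights with punches, exposing its state through Blackboard keys.
; Pawn sensing enables chase and resets a Tick-driven timer that disables it after a maximum time without sightings.
; A callable range check toggles the attack state.
; Attacks play a random montage and choose a hand by index parity, repeating a short-delay capsule trace at that hand until a hit or punch end.
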(event OnSeePawn(PawnSensing)
  (params (Pawn :type Pawn%20Object%20Reference))
  ;[1 1 1] when the enemy see's the play it chases it reset the timer. This allowsfor continous chasing until the player is not detected for the max chase time value.
  (Utilities|Casting|CastToBP_Main_Character Pawn)
  (CallFunction|EnableChase true)
  (Variables|Default|SetTimeStartChase 0.0)
  (AI|Components|Blackboard|SetValueasVector (Variables|Default|GetAI_Blackboard) (Utilities|Name|MakeLiteralName "LastKnownPosition") "0, 0, 0"))

(event Custom|OnTimerInvoke
  (CallFunction|EnableChase false))

(event Custom|CheckAttackRange
  ;[1 1 1] Combat Mechanics
  (bind _inrange (CallFunction|ComputeDistanceBetweenEnemyPlayer (Variables|Default|GetAttackRange)))
  (CallFunction|EnableAttack _inrange))

(event Custom|PerformAttack
  ;[1 1 1] Combat Mechanics
  (Variables|Default|SetIsPunching true)
  (bind (_anim_montage _arrayindex) (CallFunction|GetRandomAnimMontage))
  (if (== (Math|Integer|%(Integer) _arrayindex 2) 0)
    (Variables|Default|SetPunchingHandIndex 0)
    (else
      (Variables|Default|SetPunchingHandIndex 1)))
  (bind _returnvalue (Animation|PlayAnimMontage _anim_montage 1.0 "None"))
  (Utilities|FlowControl|Sequence
    (:then_0
      (Utilities|FlowControl|Delay _returnvalue)
      (Variables|Default|SetIsPunching false))
    (:then_1
      (CallFunction|PunchTrace))))

(event Custom|Clear%20Black%20Board%20Value
  (params (Name :type String))
  (AI|Components|Blackboard|ClearValue (Variables|Default|GetAI_Blackboard) (Utilities|Name|MakeLiteralName (Utilities|String|StringToName Name))))

(event Custom|PunchTrace
  (bind _mesh (Variables|Character|GetMesh))
  (bind _punchinghandindex (Variables|Default|GetPunchingHandIndex))
  (bind _returnvalue (Utilities|Select :Index _punchinghandindex :Option%200 "hand_l" :Option%201 "hand_r"))
  (bind _returnvalue_2 (Transformation|GetSocketLocation _mesh _returnvalue))
  ;[1 1 1] Combat Mechanics
  (if (Variables|Default|GetIsPunching)
    (bind (_outhit _returnvalue_3) (Class|KismetSystemLibrary|CapsuleTraceSingleforObjects _returnvalue_2 _returnvalue_2 22.0 22.0 (Utilities|Array|MakeArray "ObjectTypeQuery1") false 0 "None" true))
    (if _returnvalue_3
      (bind _asbp_main_character (Utilities|Casting|CastToBP_Main_Character (.HitActor (Collision|BreakHitResult _outhit))))
      (Default|RecievePunch _asbp_main_character (Variables|Default|GetPunchingHandIndex))
      (else
        (Utilities|FlowControl|Delay 0.01)
        (CallFunction|PunchTrace)))))

(event EventTick
  (params (DeltaSeconds :type Float%20%28single-precision%29))
  (CallFunction|UpdateChaseTimer DeltaSeconds))

(event EventBeginPlay
  ;[1 1 1] Caching of AI data
  (Variables|Default|SetAI_Blackboard (AI|GetBlackboard (AI|GetAIController self)))
  (Variables|Default|SetPlayer (Game|GetPlayerCharacter 0)))

(fn ConstructionScript)

(fn UpdateChaseTimer
  (params (DeltaTime :type Float%20%28double-precision%29))
  (bind _output_get (Variables|Default|SetTimeStartChase (+ DeltaTime (Variables|Default|GetTimeStartChase))))
  (if (>= _output_get (Variables|Default|GetChaseMaxTime))
    (CallFunction|OnTimerInvoke)))

(fn EnableChase
  (params (Enable :type Boolean))
  (AI|Components|Blackboard|SetValueasBool (Variables|Default|GetAI_Blackboard) (Utilities|Name|MakeLiteralName "IsPlayerDetected") Enable))

(fn EnableAttack
  (params (Enable :type Boolean))
  (AI|Components|Blackboard|SetValueasBool (Variables|Default|GetAI_Blackboard) (Utilities|Name|MakeLiteralName "IsInAttackRange") Enable)
  (Variables|Default|SetIsFighting Enable))

(fn ComputeDistanceBetweenEnemyPlayer
  (params (Range :type Float%20%28double-precision%29))
  (return (< (Math|Vector|VectorLength (- (Transformation|GetActorLocation (Variables|Default|GetPlayer)) (Transformation|GetActorLocation))) Range)))

(fn GetRandomAnimMontage
  (bind _animmontagearray (Variables|AttackAnimations|GetAnimMontageArray))
  (bind _returnvalue (Utilities|Array|Length _animmontagearray))
  (bind _returnvalue_2 (- _returnvalue 1))
  (bind _returnvalue_3 (Math|Random|RandomIntegerinRange 0 _returnvalue_2))
  (return (Utilities|Array|Get(acopy) _animmontagearray _returnvalue_3) _returnvalue_3))